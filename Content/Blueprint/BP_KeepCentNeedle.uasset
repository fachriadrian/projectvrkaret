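; BP_KeepCentNeedle is a grabbable VR needle that slides along a constrained axis and can trigger a level change.
; On grab, a fast looping timer runs ReplicatePosition until drop, moving Box along local Y to follow the motion controller.
; That movement is clamped between the first two spline points.
; When Box1 begins overlapping a BP_KeepCentNeedle actor, it opens the 5aTransferAscites level.
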(event `self.GrabComponent.OnGrabbed`
  (params (MotionController :type "MotionControllerComponent Object Reference"))
  (set `self.Motion Controller` MotionController)
  (bind _returnvalue (`KismetSystemLibrary.K2_SetTimer` null "ReplicatePosition" 0.01 true))
  (set `self.Timer` _returnvalue))

(event `self.GrabComponent.OnDropped`
  (`KismetSystemLibrary.K2_ClearAndInvalidateTimerHandle` (`self.Timer`))
  (set `self.Motion Controller` null))

(event `self.Box1.OnComponentBeginOverlap`
  (params (OverlappedComponent :type "PrimitiveComponent Object Reference") (OtherActor :type "Actor Object Reference") (OtherComp :type "PrimitiveComponent Object Reference") (OtherBodyIndex :type Integer) (bFromSweep :type Boolean) (SweepResult :type "HitResult Structure (by ref)"))
  (cast `/Game/Blueprint/BP_KeepCentNeedle` OtherActor)
  (`GameplayStatics.OpenLevelBySoftObjectPtr` "/Game/VRTemplate/Maps/5a-TransferAscites.5a-TransferAscites"))

(fn `ReplicatePosition`
  (bind _spline (`self.Spline`))
  (bind (_returnvalue_x _returnvalue_y) (`KismetMathLibrary.BreakVector` (`SplineComponent.GetLocationAtSplinePoint` _spline 0 "Local")))
  (bind (_returnvalue_x_2 _returnvalue_y_2) (`KismetMathLibrary.BreakVector` (`SplineComponent.GetLocationAtSplinePoint` _spline 1 "Local")))
  (bind (_relativelocation_x _relativelocation_y) (`KismetMathLibrary.BreakVector` (`SceneComponent.RelativeLocation` (`self.Box`))))
  (`SceneComponent.K2_SetRelativeLocation` (`self.Box`) (`KismetMathLibrary.MakeVector` 0.0 (`KismetMathLibrary.FClamp` (+ (.y (.location (`KismetMathLibrary.MakeRelativeTransform` (`SceneComponent.K2_GetComponentToWorld` (`self.Motion Controller`)) (`SceneComponent.K2_GetComponentToWorld` (`self.Box`))))) _relativelocation_y) _returnvalue_y _returnvalue_y_2)) false false))

(fn `UserConstructionScript`)
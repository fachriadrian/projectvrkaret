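; Actor that shows the HasilUSGFalse component, apparently an ultrasound (USG) result, while the transducer is in its zone.
; The component is hidden on BeginPlay through the ChangeComponentVisibility event.
; Box begin and end overlaps call that event to show or hide it, responding only to BP_USG-Transducer actors.
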(event `ChangeComponentVisibility`
  (params (`Visible?` :type Boolean))
  (`SceneComponent.SetVisibility` (`self.HasilUSGFalse`) `Visible?` (`self.Propagate to Children`)))

(event `self.ReceiveBeginPlay`
  (`self.ChangeComponentVisibility` false))

(event `self.Box.OnComponentBeginOverlap`
  (params (OverlappedComponent :type "PrimitiveComponent Object Reference") (OtherActor :type "Actor Object Reference") (OtherComp :type "PrimitiveComponent Object Reference") (OtherBodyIndex :type Integer) (bFromSweep :type Boolean) (SweepResult :type "HitResult Structure (by ref)"))
  (cast `/Game/Blueprint/BP_USG-Transducer` OtherActor)
  (`self.ChangeComponentVisibility` true))

(event `self.Box.OnComponentEndOverlap`
  (params (OverlappedComponent :type "PrimitiveComponent Object Reference") (OtherActor :type "Actor Object Reference") (OtherComp :type "PrimitiveComponent Object Reference") (OtherBodyIndex :type Integer))
  (cast `/Game/Blueprint/BP_USG-Transducer` OtherActor)
  (`self.ChangeComponentVisibility` false))

(fn `UserConstructionScript`)